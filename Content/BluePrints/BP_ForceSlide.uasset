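; BP_ForceSlide is a trigger volume that switches encounter enemies and spawners on while the first-person character is inside its box.
; Overlap begin and end call ActivateSpawners and WakeBaddies, which activate or deactivate the Spawners and Enemies arrays, gated by SpawnEnemies and WakeEnemies, and remove invalid entries.
; Shortly after BeginPlay it deactivates the enemies.
; The ForceSlide event is also called on overlap but is empty.
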(event `self.ReceiveBeginPlay`
  (`KismetSystemLibrary.Delay` 0.5)
  (`self.wakeBaddies` false))

(event `self.Box.OnComponentBeginOverlap`
  (params (OverlappedComponent :type "PrimitiveComponent Object Reference") (OtherActor :type "Actor Object Reference") (OtherComp :type "PrimitiveComponent Object Reference") (OtherBodyIndex :type Integer) (bFromSweep :type Boolean) (SweepResult :type "HitResult Structure (by ref)"))
  (cast `/Game/FirstPerson/Blueprints/BP_FirstPersonCharacter` OtherActor)
  (`self.ActivateSpawners` true)
  (`self.Force Slide` true)
  (`self.wakeBaddies` true))

(event `self.Box.OnComponentEndOverlap`
  (params (OverlappedComponent :type "PrimitiveComponent Object Reference") (OtherActor :type "Actor Object Reference") (OtherComp :type "PrimitiveComponent Object Reference") (OtherBodyIndex :type Integer))
  (cast `/Game/FirstPerson/Blueprints/BP_FirstPersonCharacter` OtherActor)
  (`self.ActivateSpawners` false)
  (`self.Force Slide` false)
  (`self.wakeBaddies` false))

(event `ActivateSpawners`
  (params (On :type Boolean))
  (bind _spawners (`self.Spawners`))
  (if (`self.SpawnEnemies`)
    (for (_array_element _array_index) _spawners
      (if (`KismetSystemLibrary.IsValid` _array_element)
        (if On
          (`/Game/BluePrints/Enemys/BP_EnemySpawner.Activate` _array_element)
          (else
            (`/Game/BluePrints/Enemys/BP_EnemySpawner.Deactivate` _array_element)))
        (else
          (`KismetArrayLibrary.Array_Remove` _spawners _array_index))))))

(event `Force Slide`
  (params (On :type Boolean)))

(event `wakeBaddies`
  (params (On :type Boolean))
  (bind _enemies (`self.Enemies`))
  (if (`self.WakeEnemies`)
    (for (_array_element _array_index) _enemies
      (if (`KismetSystemLibrary.IsValid` _array_element)
        (if On
          (`/Game/BluePrints/ParentBPs/BP_EnemyCharacter.Activate` _array_element)
          (else
            (`/Game/BluePrints/ParentBPs/BP_EnemyCharacter.Deactivate` _array_element)))
        (else
          (`KismetArrayLibrary.Array_Remove` _enemies _array_index))))))

(fn `IsValid`
  (params (TargetArray :type "Array of /Game/BluePrints/Enemys/BP_EnemySpawner Object Reference (by ref)") (Object :type "Object Object Reference") (IndexToRemove :type Integer)))

(fn `UserConstructionScript`)