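; Parent enemy character Blueprint that spots the player by distance, chases and melee-attacks, and returns home when it loses sight.
; Tick drives detection and head tracking, while MovementCheck loops between AI MoveTo pursuit and returning to its start location.
; Attacks use timeline squash-stretch and a sphere trace, and damage can rescale the body by health.
; On death, body and head launch as physics objects, then burst and shrink away, with empty AttackAnim and Flail events.
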(event `self.ReceiveBeginPlay`
  (set `self.StartLocation` (`SceneComponent.K2_GetComponentLocation` (`self.CapsuleComponent`)))
  (`KismetSystemLibrary.Delay` 0.2)
  (set `self.Localhealth` (`self.Max Health`))
  (if (`self.ISActive`)
    (if (`self.CanMove`)
      (`self.MovementCheck`))))

(event `Activate`
  (set `self.ISActive` true)
  (if (`self.CanMove`)
    (`self.MovementCheck`)))

(event `Deactivate`
  (set `self.ISActive` false)
  (set `self.Can see player` false))

(event `self.ReceiveTick`
  (params (DeltaSeconds :type "Float (single-precision)"))
  (bind _head (`self.Head`))
  (bind _returnvalue (`SceneComponent.K2_GetComponentLocation` (`self.Head`)))
  (bind _returnvalue_location (`KismetMathLibrary.BreakTransform` (`self.GetTransform` (`GameplayStatics.GetPlayerPawn` 0))))
  ; Vision
  (if (`self.ISActive`)
    (if (`self.CanLookAround`)
      (if (< (`KismetMathLibrary.Vector_Distance` (`SceneComponent.K2_GetComponentLocation` (`self.Head`)) _returnvalue_location) (`self.ViewDistance`))
        (if (`self.Can see player`)
          ; Head Turning
          (if (`self.CanLookAround`)
            (`SceneComponent.K2_SetWorldRotation` _head (`KismetMathLibrary.RLerp` (`self.Last Look Rot`) (`KismetMathLibrary.FindLookAtRotation` (`SceneComponent.K2_GetComponentLocation` _head) (`PlayerCameraManager.GetCameraLocation` (`GameplayStatics.GetPlayerCameraManager` 0))) (`self.LookBlend`) true) false false))
          (else
            (set `self.Can see player` true)
            (`self.Jump`)
            (`GameplayStatics.PlaySoundAtLocation` (`self.SpotSound`) _returnvalue (struct) 1.0 1.0 0.0 null null null null)
            (`NiagaraFunctionLibrary.SpawnSystemAtLocation` "/Game/VFX/NS_Suprise.NS_Suprise" _returnvalue)
            (`self.PauseLook` 0.3)))
        (else
          (set `self.Can see player` false))))))

(event `PauseLook`
  (params (Time :type "Float (double-precision)" :default 2.0))
  (bind _returnvalue (* Time 60.0))
  ; Head Turning
  (`/Engine/EditorBlueprintResources/StandardMacros.DoOnce` false :!label _label
    (:`Completed`
      (set `self.TargetLock` true)
      (set `self.Last Look Rot` (`SceneComponent.K2_GetComponentRotation` (`self.Head`)))
      (set `self.LookTimer` _returnvalue)
      (if (> (`self.LookTimer`) 0.0) :!label _label_2
        (bind _result (`/Engine/EditorBlueprintResources/StandardMacros.DecrementFloat` (`self.LookTimer`))
          (:`  `
            (set `self.LookBlend` (`KismetMathLibrary.MapRangeClamped` _result 0.0 _returnvalue 1.0))
            (`KismetSystemLibrary.DelayUntilNextTick`)
            (goto _label_2)))
        (else
          (set `self.TargetLock` false)
          (goto _label :!via `Reset`))))))

(event `BrassEject`
  (params (Scale :type "Float (double-precision)" :default 1.0))
  (bind _returnvalue (`SceneComponent.K2_GetComponentRotation` (`self.Head`)))
  ; Brass
  (`NiagaraFunctionLibrary.SpawnSystemAtLocation` "/Game/VFX/NS_Brass.NS_Brass" (+ (`SceneComponent.K2_GetComponentLocation` (`self.Head`)) (`KismetMathLibrary.GreaterGreater_VectorRotator` (`self.Brass offset`) _returnvalue)) _returnvalue (`KismetMathLibrary.Conv_DoubleToVector` Scale)))

(event `TakeDMG`
  (params (DMG :type "Float (double-precision)") (ShotFrom :type "Vector Structure") (Causer :type "Object Object Reference"))
  ; Health and damage
  (set `self.HitFrom` ShotFrom)
  (set `self.Localhealth` (`KismetMathLibrary.FTrunc` (- (`self.Localhealth`) DMG)))
  (set `self.Location` (`SceneComponent.K2_GetComponentLocation` (`self.StaticMesh`)))
  (`GameplayStatics.PlaySoundAtLocation` (`self.HurtSound`) (`self.Location`) (struct) 1.0 1.0 0.0 "/Game/Audio/SFX/Robots/attne_physical1.attne_physical1" null null null)
  (`self.UpdateHealth` (== (`GameplayStatics.GetPlayerPawn` 0) Causer)))

(event `UpdateHealth`
  (params (`killed by player` :type Boolean))
  ; Health and damage
  (if (`self.ScaleSizeByHealth`)
    (`self.Scale Size by health`))
  (if (<= (`self.Localhealth`) 0)
    (`/Engine/EditorBlueprintResources/StandardMacros.DoOnce` false
      (:`Completed`
        (if `killed by player`
          (`GameplayStatics.SpawnSoundAttached` (`self.DeathSound`) (`self.StaticMesh`) "None" (0.0 0.0 0.0) (struct) "SnapToTarget" true 1.0 1.0 0.0 null null))
        (`self.predie`)))))

(event `ReturnHome`
  ; Simple Pursue
  ;; ReturnHome
  (if (> (`self.Localhealth`) 0)
    (if (`self.AllredyHome`)
      (`KismetSystemLibrary.Delay` 0.5)
      (`self.MovementCheck`)
      (else
        (set `self.AllredyHome` (< (`KismetMathLibrary.Vector_Distance` (`SceneComponent.K2_GetComponentLocation` (`self.CapsuleComponent`)) (`self.StartLocation`)) 40.0))
        (if (> (`self.Localhealth`) 0)
          (`KismetSystemLibrary.PrintString` (`KismetStringLibrary.Concat_StrStr` (`KismetSystemLibrary.GetDisplayName` self) " was asked to go home") true true (struct :`R` 0.947852 :`B` 1.0 :`A` 1.0))
          (`|AIMoveTo` self (`self.StartLocation`) null 2.0
            (:`then`
              (`KismetSystemLibrary.Delay` 0.2)
              (`self.MovementCheck`))))))))

(event `Simple Pursue`
  (bind _returnvalue (`KismetSystemLibrary.GetDisplayName` self))
  ; Simple Pursue
  (if (> (`self.Localhealth`) 0)
    (`KismetSystemLibrary.PrintString` (`KismetStringLibrary.Concat_StrStr` _returnvalue " was asked to move.") true true (struct :`R` 0.947852 :`B` 1.0 :`A` 1.0))
    (`|AIMoveTo` self (0.0 0.0 0.0) (`GameplayStatics.GetPlayerCharacter` 0) (`self.AttackRange`)
      (:`OnSuccess`
        (`KismetSystemLibrary.PrintString` (`KismetStringLibrary.Concat_StrStr` _returnvalue " can see player."))
        (`self.Attack`))
      (:`OnFail`
        (`KismetSystemLibrary.PrintString` (`KismetStringLibrary.Concat_StrStr` _returnvalue " cannot find player"))))
    (`KismetSystemLibrary.Delay` 2.0)
    (`self.MovementCheck`)))

(event `MovementCheck`
  ; MovementCheck
  (if (`self.Can see player`)
    (`self.Simple Pursue`)
    (else
      (`self.ReturnHome`))))

(event `Attack`
  (bind _scaleoffset (`self.ScaleOffset`))
  (bind _scaleoffset_2 (`self.ScaleOffset`))
  (bind _capsulecomponent (`self.CapsuleComponent`))
  (bind _returnvalue (`SceneComponent.K2_GetComponentRotation` _capsulecomponent))
  (bind _returnvalue_2 (`SceneComponent.K2_GetComponentLocation` _capsulecomponent))
  ; Attack
  ;; Warm up
  (if (`self.Can Attack`)
    (`GameplayStatics.PlaySoundAtLocation` (`self.AttackSound`) (`SceneComponent.K2_GetComponentLocation` (`self.StaticMesh`)) (struct) 1.0 1.0 0.0 null null null null)
    (`self.AttackAnim`)
    ;;; Animation
    (bind (_direction _newtrack_0) (`Timeline|Timeline` :!via `PlayFromStart`)
      (:`Update`
        (`SceneComponent.SetRelativeScale3D` (`self.StaticMesh`) (`KismetMathLibrary.VLerp` _scaleoffset (* _scaleoffset (0.25 0.25 1.75)) _newtrack_0)))
      (:`Finished`
        (`self.Jump`)
        (if (`self.Can Attack`)
          (bind _outhit (`KismetSystemLibrary.SphereTraceSingleForObjects` (+ _returnvalue_2 (`KismetMathLibrary.GreaterGreater_VectorRotator` (20.0 0.0 0.0) _returnvalue)) (+ _returnvalue_2 (`KismetMathLibrary.GreaterGreater_VectorRotator` (`KismetMathLibrary.MakeVector` (`self.AttackRange`)) _returnvalue)) 20.0 (`self.Object Types ToHit`)))
          (bind (_bblockinghit _binitialoverlap _time _distance _location _impactpoint _normal _impactnormal _physmat _hitactor) (`GameplayStatics.BreakHitResult` _outhit))
          (`GameplayStatics.ApplyPointDamage` _hitactor 1.0 _normal _outhit null self "/Game/FirstPerson/Blueprints/Guns/DMG_Black.DMG_Black_C")
          ;; Animation
          (bind (_direction_2 _newtrack_0_2) (`Timeline|Timeline_0` :!via `PlayFromStart`)
            (:`Update`
              (`SceneComponent.SetRelativeScale3D` (`self.StaticMesh`) (`KismetMathLibrary.VLerp` _scaleoffset_2 (* _scaleoffset_2 (0.25 0.25 1.75)) _newtrack_0_2)))))))))

(event `AttackAnim`
  ; Attack
)

(event `Die`
  (bind _returnvalue (`SceneComponent.K2_GetComponentLocation` (`self.StaticMesh`)))
  ; Splat death
  (`NiagaraFunctionLibrary.SpawnSystemAtLocation` "/Game/VFX/Pack_Simple_Particle_Burst/01_Niagara_Systems/NS_Simple_Burst_Level_1.NS_Simple_Burst_Level_1" _returnvalue)
  (`GameplayStatics.PlaySoundAtLocation` (`self.CorpseSound`) _returnvalue (struct) 1.0 1.0 0.0 null null null null)
  (`KismetSystemLibrary.Delay` 0.01)
  (bind (_direction _newtrack_0) (`Timeline|Shink objects` :!via `PlayFromStart`)
    (:`Update`
      (`SceneComponent.SetRelativeScale3D` (`self.Head`) (* (`self.HeadSize`) _newtrack_0))
      (`SceneComponent.SetRelativeScale3D` (`self.StaticMesh`) (* (`self.BodySize`) _newtrack_0)))
    (:`Finished`
      (`self.K2_DestroyActor`))))

(event `predie`
  (bind _staticmesh (`self.StaticMesh`))
  (bind _launch_force (`self.Launch Force`))
  ; LaunchEnemies on death
  (`NiagaraFunctionLibrary.SpawnSystemAtLocation` "/Game/VFX/Pack_Simple_Particle_Burst/01_Niagara_Systems/NS_Simple_Burst_Level_1.NS_Simple_Burst_Level_1" (`SceneComponent.K2_GetComponentLocation` (`self.Head`)))
  (set `self.CanLookAround` false)
  (`self.Flail`)
  (if (`self.CanDie`)
    (`/Engine/EditorBlueprintResources/StandardMacros.DoOnce` false
      (:`Completed`
        (set `self.Can Attack` false)
        (`ActorComponent.K2_DestroyComponent` (`self.CapsuleComponent`))
        (`PrimitiveComponent.SetSimulatePhysics` _staticmesh true)
        (`PrimitiveComponent.SetSimulatePhysics` (`self.Head`) true)
        (`PrimitiveComponent.AddImpulse` _staticmesh (* (`self.HitFrom`) (* _launch_force -1.0)) "None" true)
        (`PrimitiveComponent.AddImpulse` (`self.Head`) (`KismetMathLibrary.MakeVector` 0.0 0.0 (* _launch_force 0.2)) "None" true)
        (`KismetSystemLibrary.Delay` 2.0)
        (`PrimitiveComponent.SetCollisionResponseToAllChannels` (`self.StaticMesh`) "ECR_Ignore")
        (`PrimitiveComponent.SetCollisionResponseToAllChannels` (`self.Head`) "ECR_Ignore")
        (set `self.CanTakeDamage` false)
        (`self.Die`)))))

(event `Flail`
  ; LaunchEnemies on death
)

(event `self.ReceiveHit`
  (params (MyComp :type "PrimitiveComponent Object Reference") (Other :type "Actor Object Reference") (OtherComp :type "PrimitiveComponent Object Reference") (bSelfMoved :type Boolean) (HitLocation :type "Vector Structure") (HitNormal :type "Vector Structure") (NormalImpulse :type "Vector Structure") (Hit :type "HitResult Structure (by ref)"))
  ; LaunchEnemies on death
  (if (not (`self.Can Attack`))
    (`GameplayStatics.ApplyPointDamage` Other 100.0 HitNormal Hit null self "/Game/FirstPerson/Blueprints/Guns/DMG_Blue.DMG_Blue_C")))

(fn `Is player over Enemy`
  (returns (IsPlayerOverEnemy :type Boolean))
  (bind _capsulecomponent (`self.CapsuleComponent`))
  (bind (_returnvalue_x _returnvalue_y _returnvalue_z) (`KismetMathLibrary.BreakVector` (`SceneComponent.K2_GetComponentLocation` _capsulecomponent)))
  (bind (_returnvalue_x_2 _returnvalue_y_2 _returnvalue_z_2) (`KismetMathLibrary.BreakVector` (`CharacterMovementComponent.GetLastUpdateLocation` (`Character.CharacterMovement` (`GameplayStatics.GetPlayerCharacter` 0)))))
  (return (> _returnvalue_z_2 (+ _returnvalue_z (`CapsuleComponent.GetScaledCapsuleHalfHeight` _capsulecomponent)))))

(fn `Scale Size by health`
  (bind _scaleoffset (`self.ScaleOffset`))
  (`SceneComponent.SetRelativeScale3D` (`self.StaticMesh`) (`KismetMathLibrary.VLerp` (* _scaleoffset (`self.Min Scale`)) (* _scaleoffset (`self.MaxScale`)) (`KismetMathLibrary.MapRangeClamped` (`KismetMathLibrary.Conv_IntToDouble` (`self.Localhealth`)) 0.0 (`KismetMathLibrary.Conv_IntToDouble` (`self.Max Health`)) 0.0 1.0)))
  (return))

(fn `UserConstructionScript`
  (bind _head (`self.Head`))
  (`PrimitiveComponent.SetCollisionResponseToChannel` (`self.CapsuleComponent`) "ECC_Camera" "ECR_Ignore")
  (set `self.ScaleOffset` (`SceneComponent.RelativeScale3D` (`self.StaticMesh`)))
  (set `self.Last Look Rot` (`SceneComponent.K2_GetComponentRotation` (`self.Head`)))
  ; Move the ViewHint
  (`SceneComponent.K2_SetWorldLocation` (`self.ViewHint`) (+ (`SceneComponent.K2_GetComponentLocation` _head) (`KismetMathLibrary.GreaterGreater_VectorRotator` (`KismetMathLibrary.MakeVector` (`self.ViewDistance`)) (`SceneComponent.K2_GetComponentRotation` _head))) false false)
  (set `self.HeadSize` (`SceneComponent.RelativeScale3D` (`self.Head`)))
  (set `self.BodySize` (`SceneComponent.RelativeScale3D` (`self.StaticMesh`)))
  (`ActorComponent.K2_DestroyComponent` (`self.Mesh`))
  (`ActorComponent.K2_DestroyComponent` (`self.ViewHint`)))