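; BP_Door is a door that lowers once a set number of button signals has arrived.
; Each SwitchOnandOff event decrements NumOfButtons, and at zero or below it plays DoorTimeline.
; The timeline lerps the Pivot's relative Z downward, with IsFast choosing between the FastPosition and DoorPosition tracks.
; The graph only plays the timeline forward, with no logic to close the door.
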(event `SwitchOnandOff`
  (bind _pivot (`self.Pivot`))
  (`/Engine/EditorBlueprintResources/StandardMacros.DecrementInt` (`self.Num of buttons`)
    (:`  `
      (if (<= (`self.Num of buttons`) 0)
        (bind (_direction _doorposition _fastposition) (`Timeline|Door Timeline`)
          (:`Update`
            (if (`self.IsFast`)
              (`SceneComponent.K2_SetRelativeLocation` _pivot (`KismetMathLibrary.MakeVector` 0.0 0.0 (`KismetMathLibrary.Lerp` 0.0 -400.0 _fastposition)) false false)
              (else
                (`SceneComponent.K2_SetRelativeLocation` _pivot (`KismetMathLibrary.MakeVector` 0.0 0.0 (`KismetMathLibrary.Lerp` 0.0 -400.0 _doorposition)) false false)))))))))

(fn `UserConstructionScript`)