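; BP_PressurePlate1 is a pressure plate switch that toggles a linked door when hit by green-type point damage.
; The damage must cast to DMG_Green, and a DoOnce lets it fire only once.
; On activation it calls SwitchOnandOff on DoorRef, reveals a point light hidden at construction, destroys its Plane component, and plays a timeline that moves the Switch mesh along Z.
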(event `self.ReceivePointDamage`
  (params (Damage :type "Float (single-precision)") (DamageType :type "DamageType Object Reference") (HitLocation :type "Vector Structure") (HitNormal :type "Vector Structure") (HitComponent :type "PrimitiveComponent Object Reference") (BoneName :type Name) (ShotFromDirection :type "Vector Structure") (InstigatedBy :type "Controller Object Reference") (DamageCauser :type "Actor Object Reference") (HitInfo :type "HitResult Structure (by ref)"))
  (cast `/Game/FirstPerson/Blueprints/Guns/DMG_Green` DamageType)
  (`/Engine/EditorBlueprintResources/StandardMacros.DoOnce` false
    (:`Completed`
      (`/Game/BluePrints/Door/BP_Door.SwitchOnandOff` (`self.DoorRef`))
      (`SceneComponent.SetVisibility` (`self.PointLight`) true false)
      (`ActorComponent.K2_DestroyComponent` (`self.Plane`))
      (bind (_direction _switchposition) (`Timeline|PlateTimeline` :!via `PlayFromStart`)
        (:`Update`
          (`SceneComponent.K2_SetRelativeLocation` (`self.Switch`) (`KismetMathLibrary.MakeVector` 0.0 0.0 (`KismetMathLibrary.Lerp` 0.0 0.5 _switchposition)) false false))))))

(fn `UserConstructionScript`
  (`SceneComponent.SetVisibility` (`self.PointLight`) false false))