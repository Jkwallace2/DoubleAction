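; BP_Satalite is a destructible satellite actor that breaks apart when it takes point damage of the DMG_Red type.
; The hit plays a sound, spawns an explosion, attaches smoke trails to some Rocket parts, destroys the capsule and plane, and enables physics on all Rocket pieces.
; After a short delay, a timeline drives the scale of the loose pieces, then the actor destroys itself.
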(event `self.ReceiveBeginPlay`
  (`parent.ReceiveBeginPlay`)
  (set `self.overide` true))

(event `self.ReceivePointDamage`
  (params (Damage :type "Float (single-precision)") (DamageType :type "DamageType Object Reference") (HitLocation :type "Vector Structure") (HitNormal :type "Vector Structure") (HitComponent :type "PrimitiveComponent Object Reference") (BoneName :type Name) (ShotFromDirection :type "Vector Structure") (InstigatedBy :type "Controller Object Reference") (DamageCauser :type "Actor Object Reference") (HitInfo :type "HitResult Structure (by ref)"))
  (bind _rocket (`self.Rocket`))
  (bind _returnvalue (`SceneComponent.K2_GetComponentLocation` (`self.Capsule`)))
  (cast `/Game/FirstPerson/Blueprints/Guns/DMG_Red` DamageType)
  (`GameplayStatics.PlaySoundAtLocation` "/Game/Audio/SFX/Guns/ToyTank.ToyTank" _returnvalue (struct) 1.0 0.5 0.5 null null null null)
  (`NiagaraFunctionLibrary.SpawnSystemAtLocation` "/Niagara/DefaultAssets/Templates/Systems/SimpleExplosion.SimpleExplosion" _returnvalue)
  (`NiagaraFunctionLibrary.SpawnSystemAttached` "/Game/VFX/NS_FollowSmoke.NS_FollowSmoke" (`self.Rocket`) "Socket" (0.0 0.0 0.0) (struct) "KeepRelativeOffset" true)
  (`NiagaraFunctionLibrary.SpawnSystemAttached` "/Game/VFX/NS_FollowSmoke.NS_FollowSmoke" (`self.Rocket3`) "Socket" (0.0 0.0 0.0) (struct) "KeepRelativeOffset" true)
  (`NiagaraFunctionLibrary.SpawnSystemAttached` "/Game/VFX/NS_FollowSmoke.NS_FollowSmoke" (`self.Rocket2`) "Socket" (0.0 0.0 0.0) (struct) "KeepRelativeOffset" true)
  (`NiagaraFunctionLibrary.SpawnSystemAttached` "/Game/VFX/NS_FollowSmoke.NS_FollowSmoke" (`self.Rocket1`) "Socket" (0.0 0.0 0.0) (struct) "KeepRelativeOffset" true)
  (`NiagaraFunctionLibrary.SpawnSystemAttached` "/Game/VFX/NS_FollowSmoke.NS_FollowSmoke" (`self.Rocket5`) "Socket" (0.0 0.0 0.0) (struct) "KeepRelativeOffset" true)
  (`ActorComponent.K2_DestroyComponent` (`self.Capsule`))
  (`ActorComponent.K2_DestroyComponent` (`self.Plane`))
  (`PrimitiveComponent.SetSimulatePhysics` _rocket true)
  (`PrimitiveComponent.SetSimulatePhysics` (`self.Rocket6`) true)
  (`PrimitiveComponent.SetSimulatePhysics` (`self.Rocket5`) true)
  (`PrimitiveComponent.SetSimulatePhysics` (`self.Rocket4`) true)
  (`PrimitiveComponent.SetSimulatePhysics` (`self.Rocket3`) true)
  (`PrimitiveComponent.SetSimulatePhysics` (`self.Rocket2`) true)
  (`PrimitiveComponent.SetSimulatePhysics` (`self.Rocket1`) true)
  (`PrimitiveComponent.SetSimulatePhysics` (`self.Rocket7`) true)
  (`KismetSystemLibrary.Delay` 4.0)
  (bind (_direction _newtrack_0) (`Timeline|Timeline` :!via `PlayFromStart`)
    (:`Update`
      (`SceneComponent.SetRelativeScale3D` (`self.Rocket6`) (`KismetMathLibrary.Conv_DoubleToVector` _newtrack_0))
      (`SceneComponent.SetRelativeScale3D` (`self.Rocket5`) (`KismetMathLibrary.Conv_DoubleToVector` _newtrack_0))
      (`SceneComponent.SetRelativeScale3D` (`self.Rocket4`) (`KismetMathLibrary.Conv_DoubleToVector` _newtrack_0))
      (`SceneComponent.SetRelativeScale3D` (`self.Rocket3`) (`KismetMathLibrary.Conv_DoubleToVector` _newtrack_0))
      (`SceneComponent.SetRelativeScale3D` (`self.Rocket2`) (`KismetMathLibrary.Conv_DoubleToVector` _newtrack_0))
      (`SceneComponent.SetRelativeScale3D` (`self.Rocket1`) (`KismetMathLibrary.Conv_DoubleToVector` _newtrack_0))
      (`SceneComponent.SetRelativeScale3D` (`self.Rocket7`) (`KismetMathLibrary.Conv_DoubleToVector` _newtrack_0))
      (`SceneComponent.SetRelativeScale3D` _rocket (`KismetMathLibrary.Conv_DoubleToVector` (* _newtrack_0 3.5))))
    (:`Finished`
      (`self.K2_DestroyActor`))))

(fn `UserConstructionScript`
  (`parent.UserConstructionScript`))