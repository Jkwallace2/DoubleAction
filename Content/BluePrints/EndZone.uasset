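; EndZone is the end-of-game trigger volume that finishes the game when the chicken player enters its box.
; On overlap it calls GameEndCheckpoint on the player with the transform of the BP_EndLocation found at BeginPlay.
; It then adds an audio component and, after a short delay, shows the thanks-for-playing widget with UI-only input.
; A separate ShowEndZone event blends the camera view to a given Player after a delay.
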(event `self.ReceiveBeginPlay`
  (bind _outactors (`GameplayStatics.GetAllActorsOfClass` "/Game/BluePrints/BP_EndLocation.BP_EndLocation_C"))
  (set `self.End` (`|GetArrayItem` _outactors)))

(event `self.Box.OnComponentBeginOverlap`
  (params (OverlappedComponent :type "PrimitiveComponent Object Reference") (OtherActor :type "Actor Object Reference") (OtherComp :type "PrimitiveComponent Object Reference") (OtherBodyIndex :type Integer) (bFromSweep :type Boolean) (SweepResult :type "HitResult Structure (by ref)"))
  (bind _returnvalue (`GameplayStatics.GetPlayerController` 0))
  (bind _asbp_chicken_player (cast `/Game/ChickenGame/BluePrints/BP_ChickenPlayer` OtherActor))
  (`/Game/ChickenGame/BluePrints/BP_ChickenPlayer.GameEndCheckpoint` _asbp_chicken_player (`self.GetTransform` (`self.End`)))
  (bind _returnvalue_2 (`|CreateWidget` "/Game/ChickenGame/Widgets/W_ThanksFOrPlay.W_ThanksFOrPlay_C"))
  (`AddComponent|NODE_AddAudioComponent-0` :!label _label)
  (`KismetSystemLibrary.Delay` 0.5)
  (`UserWidget.AddToViewport` _returnvalue_2 0)
  (set `PlayerController.bShowMouseCursor` true _returnvalue)
  (`WidgetBlueprintLibrary.SetInputMode_UIOnlyEx` _returnvalue null)
  (`/Engine/EditorBlueprintResources/StandardMacros.DoOnce` false
    (:`Completed`
      (goto _label))))

(event `ShowEndZone`
  (params (Player :type "Actor Object Reference"))
  (`KismetSystemLibrary.Delay` 3.0)
  (`PlayerController.SetViewTargetWithBlend` (`GameplayStatics.GetPlayerController` 0) Player 1.0 "VTBlend_Linear" 0.0 false))

(fn `UserConstructionScript`)