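; Destructible enemy spawner that, while active, sends out waves of BP_Enemy_Blue.
; Tick prunes invalid enemies from its tracked list and requests a new batch when the list empties.
; A Timeline animates a preview mesh outward with light and sound, spawns the enemy, then reverses and chains the next spawn.
; Only DMG_Blue point damage destroys it, with an explosion; other point damage shows a no-effect particle.
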(event `self.ReceiveBeginPlay`
  (`LightComponent.SetIntensity` (`self.PointLight`) 0.0)
  (`SceneComponent.SetVisibility` (`self.EnemyMesh`) false false))

(event `Check list`
  (bind _listofenemies (`self.listofenemies`))
  ; Check list
  (for (_array_element _array_index) _listofenemies
    (if (not (`KismetSystemLibrary.IsValid` _array_element))
      (`KismetArrayLibrary.Array_Remove` _listofenemies _array_index))))

(event `self.ReceiveTick`
  (params (DeltaSeconds :type "Float (single-precision)"))
  (if (`self.is Active`)
    (`self.Check list`)
    (if (<= (`KismetArrayLibrary.Array_Length` (`self.listofenemies`)) 0)
      (set `self.enemiestospawn` 5)
      (`self.SpawnEnemy`))))

(event `Activate`
  (set `self.is Active` true))

(event `Deactivate`
  (set `self.is Active` false))

(event `SpawnEnemy`
  (bind _enemiestospawn (`self.enemiestospawn`))
  (bind (_returnvalue_location _returnvalue_rotation _returnvalue_scale) (`KismetMathLibrary.BreakTransform` (`SceneComponent.K2_GetComponentToWorld` (`self.DefaultSceneRoot`))))
  (bind _returnvalue_location_2 (`KismetMathLibrary.BreakTransform` (`SceneComponent.K2_GetComponentToWorld` (`self.EnemyMesh`))))
  ; SpawnEnemy
  (if (> _enemiestospawn 0)
    (`/Engine/EditorBlueprintResources/StandardMacros.DecrementInt` _enemiestospawn
      (:`  `
        (`self.Check list`)
        (if (not (`self.IsCurentlySpawning`))
          (set `self.IsCurentlySpawning` true)
          (`GameplayStatics.PlaySoundAtLocation` "/Engine/EditorSounds/GamePreview/StartSimulate_Cue.StartSimulate_Cue" (`SceneComponent.K2_GetComponentLocation` (`self.DefaultSceneRoot`)) (struct) 2.0 1.0 0.0 "/Game/Audio/SFX/Robots/attne_physical1.attne_physical1" null null null)
          (`SceneComponent.SetVisibility` (`self.EnemyMesh`) true false)
          (`LightComponent.SetIntensity` (`self.PointLight`) 5000.0)
          (bind (_direction _newtrack_0 _newtrack_1) (`Timeline|Timeline` :!via `PlayFromStart` :!label _label)
            (:`Update`
              ;; Animation
              (`SceneComponent.K2_SetRelativeLocation` (`self.SM_Cubeend`) (`KismetMathLibrary.MakeVector` 0.0 0.0 (* _newtrack_0 (`self.offset`))) false false)
              (`SceneComponent.K2_SetRelativeLocation` (`self.EnemyMesh`) (`KismetMathLibrary.MakeVector` (`KismetMathLibrary.MapRangeClamped` _newtrack_1 0.0 1.0 -33.0 200.0) 0.0 -286.37507) false false))
            (:`Finished`
              (switch `ETimelineDirection` _direction
                (:`Forward`
                  (bind _returnvalue (`|SpawnActorFromClass` "/Game/BluePrints/Enemys/BP_Enemy_Blue.BP_Enemy_Blue_C" (`KismetMathLibrary.MakeTransform` _returnvalue_location_2 _returnvalue_rotation _returnvalue_scale) "AdjustIfPossibleButAlwaysSpawn" "MultiplyWithRoot" null null))
                  (`KismetArrayLibrary.Array_Add` (`self.listofenemies`) _returnvalue)
                  (`SceneComponent.SetVisibility` (`self.EnemyMesh`) false false)
                  (`SceneComponent.K2_SetRelativeLocation` (`self.EnemyMesh`) (-33.0 0.0 -286.37507) false false)
                  (goto _label :!via `ReverseFromEnd`))
                (:`Backward`
                  (`LightComponent.SetIntensity` (`self.PointLight`) 0.0)
                  (set `self.IsCurentlySpawning` false)
                  (`self.SpawnEnemy`))))))))))

(event `self.ReceivePointDamage`
  (params (Damage :type "Float (single-precision)") (DamageType :type "DamageType Object Reference") (HitLocation :type "Vector Structure") (HitNormal :type "Vector Structure") (HitComponent :type "PrimitiveComponent Object Reference") (BoneName :type Name) (ShotFromDirection :type "Vector Structure") (InstigatedBy :type "Controller Object Reference") (DamageCauser :type "Actor Object Reference") (HitInfo :type "HitResult Structure (by ref)"))
  (cast `/Game/FirstPerson/Blueprints/Guns/DMG_Blue` DamageType
    (:`then`
      (`self.Die`))
    (:`CastFailed`
      (`NiagaraFunctionLibrary.SpawnSystemAtLocation` "/Game/VFX/NS_Noeffect.NS_Noeffect" (+ (`SceneComponent.K2_GetComponentLocation` (`self.SM_Cubeend`)) (0.0 0.0 80.0)) (struct) (1.0 1.0 1.0) true true "None" false))))

(event `telefrag`
  (bind _defaultsceneroot (`self.DefaultSceneRoot`))
  (bind _returnvalue (`SceneComponent.K2_GetComponentLocation` _defaultsceneroot))
  (bind _outhit (`KismetSystemLibrary.SphereTraceSingleByProfile` :`Start` _returnvalue :`End` (+ _returnvalue (`KismetMathLibrary.GreaterGreater_VectorRotator` (80.0 0.0 0.0) (`SceneComponent.K2_GetComponentRotation` _defaultsceneroot))) :`Radius` 60.0 :`ProfileName` "Pawn" :`DrawDebugType` "ForDuration"))
  (bind (_bblockinghit _binitialoverlap _time _distance _location _impactpoint _normal _impactnormal _physmat _hitactor) (`GameplayStatics.BreakHitResult` _outhit))
  (`GameplayStatics.ApplyPointDamage` _hitactor 1.0 _impactpoint _outhit))

(event `Die`
  (bind (_returnvalue_location _returnvalue_rotation) (`KismetMathLibrary.BreakTransform` (`SceneComponent.K2_GetComponentToWorld` (`self.DefaultSceneRoot`))))
  (`/Engine/EditorBlueprintResources/StandardMacros.DoOnce` false
    (:`Completed`
      (set `self.is Active` false)
      (set `self.isRedyTospawn` false)
      (set `self.IsCurentlySpawning` true)
      (`GameplayStatics.PlaySoundAtLocation` "/Game/Audio/SFX/Guns/ToyRailGun.ToyRailGun" _returnvalue_location (struct) 1.0 0.8 0.0 "/Game/Audio/SFX/Robots/attne_physical1.attne_physical1" null null null)
      (`NiagaraFunctionLibrary.SpawnSystemAtLocation` "/Niagara/DefaultAssets/Templates/Systems/SimpleExplosion.SimpleExplosion" _returnvalue_location _returnvalue_rotation)
      (`self.K2_DestroyActor`))))

(fn `SpawnXEnemy`
  (params (Num :type Integer :default 5))
  (returns (Finished :type Boolean))
  (locals (i :type Integer))
  (set `self.isRedyTospawn` false)
  (set `local.i` Num)
  (while (> (`local.i`) 0)
    (`/Engine/EditorBlueprintResources/StandardMacros.DecrementInt` (`local.i`)
      (:`  `
        (`self.SpawnEnemy`)
        (`self.Check list`))))
  (return true))

(fn `UserConstructionScript`)