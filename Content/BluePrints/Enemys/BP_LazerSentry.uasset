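; BP_LazerSentry is a stationary enemy sentry that shoots at the player when they cross its forward line of sight.
; Each Tick, while able to shoot, it sphere-traces along the capsule's facing out to near ViewDistance, looking for BP_FirstPersonCharacter.
; A hit triggers sound, a light flash, brass ejection and a delayed BP_EnemyBullet spawn, with DoOnce and CanShoot enforcing a cooldown.
; BeginPlay disables movement and briefly draws a red debug sight line.
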(event `self.ReceiveBeginPlay`
  (bind _capsulecomponent (`self.CapsuleComponent`))
  (bind _returnvalue (`SceneComponent.K2_GetComponentLocation` _capsulecomponent))
  (`parent.ReceiveBeginPlay`)
  (set `self.CanMove` false)
  (`KismetSystemLibrary.DrawDebugLine` _returnvalue (+ _returnvalue (`KismetMathLibrary.GreaterGreater_VectorRotator` (`KismetMathLibrary.MakeVector` (`self.ViewDistance`)) (`SceneComponent.K2_GetComponentRotation` _capsulecomponent))) (struct :`R` 1.0 :`G` 0.062022 :`A` 1.0) 10.0 10.0))

(event `self.ReceiveTick`
  (params (DeltaSeconds :type "Float (single-precision)"))
  (bind _capsulecomponent (`self.CapsuleComponent`))
  (bind _capsulecomponent_2 (`self.CapsuleComponent`))
  (bind _pointlight (`self.PointLight`))
  (bind _returnvalue (`SceneComponent.K2_GetComponentRotation` _capsulecomponent))
  (bind _returnvalue_2 (`SceneComponent.K2_GetComponentRotation` _capsulecomponent_2))
  (if (`self.CanShoot`)
    (bind _outhit (`KismetSystemLibrary.SphereTraceSingleForObjects` (+ (`SceneComponent.K2_GetComponentLocation` (`self.CapsuleComponent`)) (`KismetMathLibrary.GreaterGreater_VectorRotator` (50.0 0.0 0.0) _returnvalue)) (+ (`SceneComponent.K2_GetComponentLocation` _capsulecomponent) (`KismetMathLibrary.GreaterGreater_VectorRotator` (`KismetMathLibrary.MakeVector` (- (`self.ViewDistance`) 80.0)) _returnvalue)) 80.0 (`self.Object Types`)))
    (`/Engine/EditorBlueprintResources/StandardMacros.DoOnce` false :!label _label
      (:`Completed`
        (cast `/Game/FirstPerson/Blueprints/BP_FirstPersonCharacter` (`.HitActor` (`GameplayStatics.BreakHitResult` _outhit))
          (:`then`
            (set `self.CanShoot` false)
            (`LightComponent.SetIntensity` _pointlight 8.0)
            (`GameplayStatics.PlaySoundAtLocation` "/Game/Audio/SFX/Guns/ToyMachineGun1.ToyMachineGun1" (`SceneComponent.K2_GetComponentLocation` (`self.CapsuleComponent`)) (struct) 1.0 0.8 0.1 null null null null) ; Play firing sound
            (`KismetSystemLibrary.Delay` 0.2)
            (`LightComponent.SetIntensity` _pointlight 0.0)
            (`self.BrassEject` 1.0)
            (`|SpawnActorFromClass` "/Game/BluePrints/Enemys/BP_EnemyBullet.BP_EnemyBullet_C" (`KismetMathLibrary.MakeTransform` (+ (`SceneComponent.K2_GetComponentLocation` _capsulecomponent_2) (`KismetMathLibrary.GreaterGreater_VectorRotator` (`self.Projectile Offset`) _returnvalue_2)) _returnvalue_2) "AlwaysSpawn" "OverrideRootScale" self null)
            (`KismetSystemLibrary.Delay` 1.0)
            (set `self.CanShoot` true)
            (goto _label :!via `Reset`))
          (:`CastFailed`
            (goto _label :!via `Reset`)))))))

(fn `UserConstructionScript`
  (`parent.UserConstructionScript`)
  (`LightComponent.SetIntensity` (`self.PointLight`) 0.0))