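; BP_TrackingSentry is a stationary enemy sentry that fires bursts of metal rounds at the player.
; While attacking is enabled, Tick traces forward from the head, and a target lock with a player hit leads to a stagger delay and look pause.
; A delayed loop, gated by DoOnce, then spawns projectiles from the head socket with sound, light flash and brass ejection.
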(event `self.ReceiveBeginPlay`
  (`parent.ReceiveBeginPlay`)
  (set `self.CanMove` false))

(event `self.ReceiveTick`
  (params (DeltaSeconds :type "Float (single-precision)"))
  (bind _head (`self.Head`))
  (bind _returnvalue (`SceneComponent.K2_GetComponentLocation` _head))
  (bind _returnvalue_2 (`SceneComponent.K2_GetComponentRotation` (`self.Head`)))
  (bind _returnvalue_3 (`SceneComponent.K2_GetComponentRotation` _head))
  (`parent.ReceiveTick` 0.0)
  (if (`self.Can Attack`)
    (bind _outhit (`KismetSystemLibrary.LineTraceSingleByProfile` :`Start` (+ _returnvalue (`KismetMathLibrary.GreaterGreater_VectorRotator` (50.0 0.0 0.0) _returnvalue_3)) :`End` (+ _returnvalue (`KismetMathLibrary.GreaterGreater_VectorRotator` (`KismetMathLibrary.MakeVector` (`self.ViewDistance`)) _returnvalue_3)) :`TraceHitColor` (struct)))
    (if (`self.TargetLock`)
      (goto _label :!via `Reset`)
      (else
        (`/Engine/EditorBlueprintResources/StandardMacros.DoOnce` false :!label _label
          (:`Completed`
            (cast `/Game/FirstPerson/Blueprints/BP_FirstPersonCharacter` (`.HitActor` (`GameplayStatics.BreakHitResult` _outhit))
              (:`then`
                (`KismetSystemLibrary.Delay` (`self.StaggerDelay`))
                (`self.PauseLook` 2.0)
                (`KismetSystemLibrary.Delay` 0.2)
                (`/Engine/EditorBlueprintResources/StandardMacros.DoOnce` false :!label _label_2
                  (:`Completed`
                    (set `self.I` (`self.ShotCount`))
                    (if (> (`self.I`) 1) :!label _label_3
                      (`/Engine/EditorBlueprintResources/StandardMacros.DecrementInt` (`self.I`)
                        (:`  `
                          (`GameplayStatics.PlaySoundAtLocation` "/Game/Audio/SFX/Guns/ToyMachineGun2.ToyMachineGun2" (`SceneComponent.GetSocketLocation` (`self.Head`) "Socket") (struct) 0.6 1.0 0.3 null null null null) ; Play firing sound
                          (`LightComponent.SetIntensity` (`self.PointLight`) 8.0)
                          (`|SpawnActorFromClass` "/Game/BluePrints/Enemys/BP_EnemyMetalRounds.BP_EnemyMetalRounds_C" (`KismetMathLibrary.MakeTransform` (+ (`SceneComponent.GetSocketLocation` (`self.Head`) "Socket") (`KismetMathLibrary.GreaterGreater_VectorRotator` (`self.Projectile Offset`) _returnvalue_2)) _returnvalue_2) "AlwaysSpawn" "OverrideRootScale" self null)
                          (`self.BrassEject` 1.0)
                          (`KismetSystemLibrary.Delay` 0.1)
                          (`LightComponent.SetIntensity` (`self.PointLight`) 0.0)
                          (goto _label_3)))
                      (else
                        (goto _label_2 :!via `Reset`))))))
              (:`CastFailed`
                (goto _label :!via `Reset`)))))))))

(fn `UserConstructionScript`
  (`parent.UserConstructionScript`)
  (`LightComponent.SetIntensity` (`self.PointLight`) 0.0)
  (set `self.CanLookAround` true)
  (set `self.Can Attack` true)
  (set `self.ShotDelay` 4.0))