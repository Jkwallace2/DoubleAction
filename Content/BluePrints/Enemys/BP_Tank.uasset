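; Tank enemy that stands still and fires BP_TankRound projectiles at the player.
; While it can attack, Tick traces along the head's facing up to view distance, with a DoOnce and target lock gating each shot.
; A trace hit on the player character pauses looking, flashes the point light with a firing sound, then after short delays spawns the round and a brass Niagara effect.
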(event `self.ReceiveBeginPlay`
  (`parent.ReceiveBeginPlay`)
  (set `self.CanMove` false))

(event `self.ReceiveTick`
  (params (DeltaSeconds :type "Float (single-precision)"))
  (bind _head (`self.Head`))
  (bind _returnvalue (`SceneComponent.K2_GetComponentLocation` (`self.Head`)))
  (bind _returnvalue_2 (`SceneComponent.K2_GetComponentRotation` (`self.Head`)))
  (bind _returnvalue_3 (`SceneComponent.K2_GetComponentRotation` _head))
  (`parent.ReceiveTick` 0.0)
  (if (`self.Can Attack`)
    (bind _outhit (`KismetSystemLibrary.LineTraceSingleByProfile` :`Start` (+ (`SceneComponent.K2_GetComponentLocation` (`self.Head`)) (`KismetMathLibrary.GreaterGreater_VectorRotator` (50.0 0.0 0.0) _returnvalue_3)) :`End` (+ (`SceneComponent.K2_GetComponentLocation` _head) (`KismetMathLibrary.GreaterGreater_VectorRotator` (`KismetMathLibrary.MakeVector` (`self.ViewDistance`)) _returnvalue_3)) :`TraceHitColor` (struct)))
    (if (`self.TargetLock`)
      (goto _label :!via `Reset`)
      (else
        (`/Engine/EditorBlueprintResources/StandardMacros.DoOnce` false :!label _label
          (:`Completed`
            (cast `/Game/FirstPerson/Blueprints/BP_FirstPersonCharacter` (`.HitActor` (`GameplayStatics.BreakHitResult` _outhit))
              (:`then`
                (`self.PauseLook` 3.0)
                (`LightComponent.SetIntensity` (`self.PointLight`) 8.0)
                (`GameplayStatics.PlaySoundAtLocation` "/Game/Audio/SFX/Guns/ToyTank3.ToyTank3" (`SceneComponent.K2_GetComponentLocation` (`self.Head`)) (struct) 2.0 1.0 0.0 null null null null) ; Play firing sound
                (`KismetSystemLibrary.Delay` 0.3)
                (`LightComponent.SetIntensity` (`self.PointLight`) 0.0)
                (`|SpawnActorFromClass` "/Game/BluePrints/Enemys/BP_TankRound.BP_TankRound_C" (`KismetMathLibrary.MakeTransform` (+ _returnvalue (`KismetMathLibrary.GreaterGreater_VectorRotator` (`self.Projectile Offset`) _returnvalue_2)) _returnvalue_2) "AlwaysSpawn" "OverrideRootScale" self null)
                (`KismetSystemLibrary.Delay` 0.1)
                (`NiagaraFunctionLibrary.SpawnSystemAtLocation` "/Game/VFX/NS_BigBrass.NS_BigBrass" _returnvalue _returnvalue_2))
              (:`CastFailed`
                (goto _label :!via `Reset`)))))))))

(fn `UserConstructionScript`
  (`parent.UserConstructionScript`)
  (`LightComponent.SetIntensity` (`self.PointLight`) 0.0)
  (set `self.ShotDelay` 3.0))