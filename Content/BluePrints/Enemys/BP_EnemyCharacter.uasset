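; Base enemy character that chases and attacks the player within a vision radius, otherwise returning to its spawn point.
; A throttled Tick distance check sets CanSeePlayer, and a self-rescheduling MovementCheck picks AIMoveTo pursuit or return home.
; Attacks use a timeline stretch and jump, then range-checked point damage whose hit direction carries knockback.
; Damage can rescale the mesh by health; at zero, an overridable Predie leads to animated death and destruction.
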(event `self.ReceiveBeginPlay`
  (set `self.StartLocation` (`SceneComponent.K2_GetComponentLocation` (`self.CapsuleComponent`)))
  (`KismetSystemLibrary.Delay` 0.2)
  (set `CharacterMovementComponent.MaxWalkSpeed` 200.0 (`self.CharacterMovement`))
  (set `self.Localhealth` (`self.Max Health`))
  (if (`self.CanMove`)
    (`self.MovementCheck`)))

(event `self.ReceiveTick`
  (params (DeltaSeconds :type "Float (single-precision)"))
  ; Vision
  (`KismetSystemLibrary.Delay` 0.2)
  (if (`self.Can Attack`)
    (if (<= (`KismetMathLibrary.Vector_Distance` (`SceneComponent.K2_GetComponentLocation` (`self.CapsuleComponent`)) (`CharacterMovementComponent.GetLastUpdateLocation` (`Character.CharacterMovement` (`GameplayStatics.GetPlayerCharacter` 0)))) (`self.VisionDiameter`))
      (if (not (`self.Can see player`))
        (set `self.Can see player` true)
        (`self.Jump`)
        (`GameplayStatics.PlaySoundAtLocation` (`self.SpotSound`) (`SceneComponent.K2_GetComponentLocation` (`self.CapsuleComponent`)) (struct) 1.0 1.0 0.0 null null null null))
      (else
        (set `self.Can see player` false)))))

(event `self.ReceiveAnyDamage`
  (params (Damage :type "Float (single-precision)") (DamageType :type "DamageType Object Reference") (InstigatedBy :type "Controller Object Reference") (DamageCauser :type "Actor Object Reference"))
  ; Health and damage
  (set `self.Localhealth` (- (`self.Localhealth`) (`KismetMathLibrary.FTrunc` Damage)))
  (`KismetSystemLibrary.PrintString` (`KismetStringLibrary.Concat_StrStr` (`KismetSystemLibrary.GetDisplayName` self) " was damaged " (`KismetStringLibrary.Conv_DoubleToString` Damage) " for " (`KismetSystemLibrary.GetDisplayName` DamageCauser)) true true (struct :`R` 1.0 :`B` 0.009844 :`A` 1.0))
  (set `self.Location` (`SceneComponent.K2_GetComponentLocation` (`self.StaticMesh`)) :!label _label)
  (`KismetSystemLibrary.PrintString` (`KismetStringLibrary.Concat_StrStr` (`KismetSystemLibrary.GetDisplayName` self) " took damage") true true (struct :`R` 0.095645 :`G` 1.0 :`A` 1.0))
  (`GameplayStatics.PlaySoundAtLocation` (`self.HurtSound`) (`self.Location`) (struct) 1.0 1.0 0.0 null null null null)
  (`self.UpdateHealth`))

(event `self.ReceivePointDamage`
  (params (Damage :type "Float (single-precision)") (DamageType :type "DamageType Object Reference") (HitLocation :type "Vector Structure") (HitNormal :type "Vector Structure") (HitComponent :type "PrimitiveComponent Object Reference") (BoneName :type Name) (ShotFromDirection :type "Vector Structure") (InstigatedBy :type "Controller Object Reference") (DamageCauser :type "Actor Object Reference") (HitInfo :type "HitResult Structure (by ref)"))
  ; Health and damage
  (`CharacterMovementComponent.AddImpulse` (`self.CharacterMovement`) ShotFromDirection true)
  (set `self.Localhealth` (`KismetMathLibrary.FTrunc` (- (`self.Localhealth`) Damage)))
  (`KismetSystemLibrary.PrintString` (`KismetStringLibrary.Concat_StrStr` (`KismetSystemLibrary.GetDisplayName` self) " was damaged " (`KismetSystemLibrary.GetDisplayName` DamageCauser) " for " (`KismetStringLibrary.Conv_DoubleToString` Damage)) true true (struct :`R` 1.0 :`B` 0.009844 :`A` 1.0))
  (goto _label))

(event `UpdateHealth`
  ; Health and damage
  (if (`self.ScaleSizeByHealth`)
    (`self.Scale Size by health`))
  (if (<= (`self.Localhealth`) 0)
    (`GameplayStatics.PlaySoundAtLocation` (`self.DeathSound`) (`self.Location`) (struct) 1.0 1.0 0.0 null null null null)
    (`self.predie`)))

(event `predie`
  ; Health and damage
  ;; Children can overide predie if they want to do something special upon death.
  (`self.Die`))

(event `ReturnHome`
  ; ReturnHome
  (if (`self.AllredyHome`)
    (`KismetSystemLibrary.Delay` 0.5)
    (`self.MovementCheck`)
    (else
      (set `self.AllredyHome` (< (`KismetMathLibrary.Vector_Distance` (`SceneComponent.K2_GetComponentLocation` (`self.CapsuleComponent`)) (`self.StartLocation`)) 40.0))
      (if (> (`self.Localhealth`) 0)
        (`KismetSystemLibrary.PrintString` (`KismetStringLibrary.Concat_StrStr` (`KismetSystemLibrary.GetDisplayName` self) " was asked to go home") true true (struct :`R` 0.947852 :`B` 1.0 :`A` 1.0))
        (`|AIMoveTo` self (`self.StartLocation`) null 2.0
          (:`then`
            (`KismetSystemLibrary.Delay` 0.2)
            (`self.MovementCheck`)))))))

(event `Simple Pursue`
  (bind _returnvalue (`KismetSystemLibrary.GetDisplayName` self))
  ; Simple Pursue
  (if (> (`self.Localhealth`) 0)
    (`KismetSystemLibrary.PrintString` (`KismetStringLibrary.Concat_StrStr` _returnvalue " was asked to move.") true true (struct :`R` 0.947852 :`B` 1.0 :`A` 1.0))
    (`|AIMoveTo` self (0.0 0.0 0.0) (`GameplayStatics.GetPlayerCharacter` 0) (`self.AttackRange`)
      (:`OnSuccess`
        (`KismetSystemLibrary.PrintString` (`KismetStringLibrary.Concat_StrStr` _returnvalue " can see player."))
        (`self.Attack`))
      (:`OnFail`
        (`KismetSystemLibrary.PrintString` (`KismetStringLibrary.Concat_StrStr` _returnvalue " cannot find player"))))
    (`KismetSystemLibrary.Delay` 2.0)
    (`self.MovementCheck`)))

(event `MovementCheck`
  ; MovementCheck
  (if (`self.Can see player`)
    (`self.Simple Pursue`)
    (else
      (`self.ReturnHome`))))

(event `Die`
  ; Death
  (if (`self.CanDie`)
    (`/Engine/EditorBlueprintResources/StandardMacros.DoOnce` false
      (:`Completed`
        (set `self.CanTakeDamage` false)
        (set `self.Can Attack` false)
        (`PrimitiveComponent.SetCollisionResponseToChannel` (`self.CapsuleComponent`) "ECC_Pawn" "ECR_Ignore")
        ;; Animation
        (bind (_direction _newtrack_0) (`Timeline|Timeline_3` :!via `PlayFromStart`)
          (:`Update`
            (`SceneComponent.SetRelativeScale3D` (`self.CapsuleComponent`) (`KismetMathLibrary.VLerp` (1.0 1.0 0.01) (* (1.0 1.0 10.0) (1.5 1.5 0.125)) _newtrack_0)))
          (:`Finished`
            (`KismetSystemLibrary.Delay` 0.5)
            ;; Death VFX
            (`NiagaraFunctionLibrary.SpawnSystemAtLocation` null (`self.Location`))
            (`GameplayStatics.PlaySoundAtLocation` (`self.CorpseSound`) (`self.Location`) (struct) 1.0 1.0 0.0 null null null null)
            (`KismetSystemLibrary.Delay` 0.01)
            (`self.K2_DestroyActor`)))))))

(event `Attack`
  (bind _scaleoffset (`self.ScaleOffset`))
  (bind _scaleoffset_2 (`self.ScaleOffset`))
  ; Attack
  ;; Warm up
  (if (`self.Can Attack`)
    (`GameplayStatics.PlaySoundAtLocation` (`self.AttackSound`) (`SceneComponent.K2_GetComponentLocation` (`self.StaticMesh`)) (struct) 1.0 1.0 0.0 null null null null)
    ;;; Animation
    (bind (_direction _newtrack_0) (`Timeline|Timeline` :!via `PlayFromStart`)
      (:`Update`
        (`SceneComponent.SetRelativeScale3D` (`self.StaticMesh`) (`KismetMathLibrary.VLerp` _scaleoffset (* _scaleoffset (0.25 0.25 1.75)) _newtrack_0)))
      (:`Finished`
        (`self.Jump`)
        (if (< (`KismetMathLibrary.Vector_Distance` (`SceneComponent.K2_GetComponentLocation` (`self.StaticMesh`)) (`CharacterMovementComponent.GetLastUpdateLocation` (`Character.CharacterMovement` (`GameplayStatics.GetPlayerCharacter` 0)))) (`self.DamageRange`))
          (`GameplayStatics.ApplyPointDamage` (`GameplayStatics.GetPlayerPawn` 0) 1.0 (* (`SceneComponent.GetForwardVector` (`self.CapsuleComponent`)) (`self.Knockback`)) (`GameplayStatics.MakeHitResult` false) null self)
          ;; Animation
          (bind (_direction_2 _newtrack_0_2) (`Timeline|Timeline_0` :!via `PlayFromStart` :!label _label_2)
            (:`Update`
              (`SceneComponent.SetRelativeScale3D` (`self.StaticMesh`) (`KismetMathLibrary.VLerp` _scaleoffset_2 (* _scaleoffset_2 (0.25 0.25 1.75)) _newtrack_0_2))))
          (else
            (goto _label_2 :!via `PlayFromStart`)))))))

(fn `Is player over Enemy`
  (returns (IsPlayerOverEnemy :type Boolean))
  (bind _manualcollision (`self.ManualCollision`))
  (bind (_returnvalue_x _returnvalue_y _returnvalue_z) (`KismetMathLibrary.BreakVector` (`BoxComponent.GetScaledBoxExtent` _manualcollision)))
  (bind (_returnvalue_x_2 _returnvalue_y_2 _returnvalue_z_2) (`KismetMathLibrary.BreakVector` (`SceneComponent.K2_GetComponentLocation` _manualcollision)))
  (bind (_returnvalue_x_3 _returnvalue_y_3 _returnvalue_z_3) (`KismetMathLibrary.BreakVector` (`CharacterMovementComponent.GetLastUpdateLocation` (`Character.CharacterMovement` (`GameplayStatics.GetPlayerCharacter` 0)))))
  (return (> _returnvalue_z_3 (+ _returnvalue_z_2 (/ _returnvalue_z 2.0)))))

(fn `Scale Size by health`
  (bind _scaleoffset (`self.ScaleOffset`))
  (`SceneComponent.SetRelativeScale3D` (`self.StaticMesh`) (`KismetMathLibrary.VLerp` (* _scaleoffset (`self.Min Scale`)) (* _scaleoffset (`self.MaxScale`)) (`KismetMathLibrary.MapRangeClamped` (`KismetMathLibrary.Conv_IntToDouble` (`self.Localhealth`)) 0.0 (`KismetMathLibrary.Conv_IntToDouble` (`self.Max Health`)) 0.0 1.0)))
  (return))

(fn `UserConstructionScript`
  (`PrimitiveComponent.SetCollisionResponseToChannel` (`self.CapsuleComponent`) "ECC_Camera" "ECR_Ignore")
  (set `self.ScaleOffset` (`SceneComponent.RelativeScale3D` (`self.StaticMesh`))))