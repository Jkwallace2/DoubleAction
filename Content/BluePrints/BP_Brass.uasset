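; BP_Brass is a coin actor that pings when spawned, waits briefly, then collects itself.
; OnSpawn plays a tone at the given pitch offset and calls Collect after a delay.
; Collect turns off physics and collision, then a timeline shrinks the coin from the scale cached in the construction script before destroying the actor.
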(event `Collect`
  (`PrimitiveComponent.SetSimulatePhysics` (`self.Coin`) false)
  (`PrimitiveComponent.SetCollisionEnabled` (`self.Capsule`) "NoCollision")
  (`PrimitiveComponent.SetCollisionEnabled` (`self.Coin`) "NoCollision")
  (bind (_direction _newtrack_1) (`Timeline|Timeline_0` :!via `PlayFromStart`)
    (:`Update`
      (`SceneComponent.SetRelativeScale3D` (`self.Coin`) (* (`KismetMathLibrary.Conv_DoubleToVector` (- 1.0 _newtrack_1)) (`self.Relative Scale 3D`))))
    (:`Finished`
      (`self.K2_DestroyActor`))))

(event `On Spawn`
  (params (PitchOffset :type "Float (double-precision)"))
  (`GameplayStatics.PlaySoundAtLocation` "/Engine/EngineSounds/1kSineTonePing.1kSineTonePing" (0.0 0.0 0.0) (struct) 0.5 PitchOffset 0.0 null null null null)
  (`KismetSystemLibrary.Delay` 2.0)
  (`self.Collect`))

(fn `UserConstructionScript`
  (set `self.Relative Scale 3D` (`SceneComponent.RelativeScale3D` (`self.Coin`))))