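; BP_Destructable is an actor that breaks on taking any damage.
; It plays a positional dodgeball sound and spawns a BP_Pinata actor at its Emitter component's location and rotation.
; The static mesh then switches to physics simulation with physics-only collision, and the actor destroys itself after a brief delay.
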(event `self.ReceiveAnyDamage`
  (params (Damage :type "Float (single-precision)") (DamageType :type "DamageType Object Reference") (InstigatedBy :type "Controller Object Reference") (DamageCauser :type "Actor Object Reference"))
  (bind _staticmesh (`self.StaticMesh`))
  (bind (_returnvalue_location _returnvalue_rotation) (`KismetMathLibrary.BreakTransform` (`SceneComponent.K2_GetComponentToWorld` (`self.Emitter`))))
  (`GameplayStatics.PlaySoundAtLocation` "/Game/Audio/Attribution/freesound/burnsie289__dodgeball.burnsie289__dodgeball" (`SceneComponent.K2_GetComponentLocation` (`self.DefaultSceneRoot`)) (struct) 0.3 0.7 0.0 "/USDCore/USDDefaultAttenuation.USDDefaultAttenuation" null null null)
  (`|SpawnActorFromClass` "/Game/MarbleGame_Wallace/BluePrints/PuzzleElements/BP_Pinata.BP_Pinata_C" (`KismetMathLibrary.MakeTransform` _returnvalue_location _returnvalue_rotation) "Undefined" "MultiplyWithRoot" null null)
  (`PrimitiveComponent.SetSimulatePhysics` _staticmesh true)
  (`PrimitiveComponent.SetCollisionEnabled` _staticmesh "PhysicsOnly")
  (`KismetSystemLibrary.Delay` 0.2)
  (`self.K2_DestroyActor`))

(fn `UserConstructionScript`)