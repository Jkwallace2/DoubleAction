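; Puzzle reset button that fires when the player character, or optionally a toy ball, overlaps its trigger box while resetting is allowed.
; It briefly swaps the button to a wait material, then resets linked spawners and puzzle elements without waiting for the delay.
; The element loop is nested in the spawner loop, so elements reset only with valid spawners and repeat for each.
; Deactivate disables resetting, and construction sets button visibility.
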(event `self.Box.OnComponentBeginOverlap`
  (params (OverlappedComponent :type "PrimitiveComponent Object Reference") (OtherActor :type "Actor Object Reference") (OtherComp :type "PrimitiveComponent Object Reference") (OtherBodyIndex :type Integer) (bFromSweep :type Boolean) (SweepResult :type "HitResult Structure (by ref)"))
  (bind _spawnerstoreset (`self.SpawnerstoReset`))
  (cast `/Game/MarbleGame_Wallace/BluePrints/PuzzleElements/BP_ToyBall` OtherActor
    (:`then`
      (if (not (`self.LookForBall_0`))
        (cast `/Game/Blueprints/BP_ThirdPersonCharacterCustom` OtherActor :!label _label) ; Did the player step on our platform?
      ))
    (:`CastFailed`
      (goto _label)))
  (if (`self.CanReset`)
    (`self.Activate`)
    (for _array_element _spawnerstoreset
      (if (`KismetSystemLibrary.IsValid` _array_element)
        (`/Game/MarbleGame_Wallace/BluePrints/PuzzleElements/BallSpawner.Reset` _spawnerstoreset)
        (for _array_element_2 (`self.ElementstoReset`)
          (if (`KismetSystemLibrary.IsValid` _array_element_2)
            (`/Game/MarbleGame_Wallace/BluePrints/PuzzleElements/BP_Element.Reset` _array_element_2)))))))

(event `Activate`
  (bind _button (`self.Button`))
  (`PrimitiveComponent.SetMaterial` _button 0 (`self.WaitMaterial`)) ; Change the color of the platform to "Activated"
  (`KismetSystemLibrary.Delay` 1.0)
  (`PrimitiveComponent.SetMaterial` _button 0 (`self.OkMaterial`)) ; Change the color of the platform to "Activated"
)

(event `Deactivate`
  (set `self.CanReset` false))

(fn `UserConstructionScript`
  (`SceneComponent.SetVisibility` (`self.Button`) (`self.Visible_0`) false)
  (`PrimitiveComponent.SetMaterial` (`self.Button`) 0 (`self.OkMaterial`)))