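; Black hole puzzle element for the marble game that pulls an overlapping BP_ToyBall toward its center.
; Entering the Outer sphere starts a 64-frame loop that applies a constant negative radial force to the ball's mesh, printing its name each pass.
; The construction script sizes both spheres from radius variables.
; Inner overlap only closes a Tick-fed gate with nothing downstream.
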(event `self.Inner.OnComponentBeginOverlap`
  (params (OverlappedComponent :type "PrimitiveComponent Object Reference") (OtherActor :type "Actor Object Reference") (OtherComp :type "PrimitiveComponent Object Reference") (OtherBodyIndex :type Integer) (bFromSweep :type Boolean) (SweepResult :type "HitResult Structure (by ref)"))
  (cast `/Game/MarbleGame_Wallace/BluePrints/PuzzleElements/BP_ToyBall` OtherActor)
  (goto _label :!via `Close`))

(event `self.ReceiveActorBeginOverlap`
  (params (OtherActor :type "Actor Object Reference")))

(event `self.ReceiveTick`
  (params (DeltaSeconds :type "Float (single-precision)"))
  (`/Engine/EditorBlueprintResources/StandardMacros.Gate` true :!label _label))

(event `self.Outer.OnComponentBeginOverlap`
  (params (OverlappedComponent :type "PrimitiveComponent Object Reference") (OtherActor :type "Actor Object Reference") (OtherComp :type "PrimitiveComponent Object Reference") (OtherBodyIndex :type Integer) (bFromSweep :type Boolean) (SweepResult :type "HitResult Structure (by ref)"))
  (bind _asbp_toy_ball (cast `/Game/MarbleGame_Wallace/BluePrints/PuzzleElements/BP_ToyBall` OtherActor))
  (set `self.Target` _asbp_toy_ball)
  (bind _output_get (set `self.X` 0))
  (while (< _output_get 64)
    (set `self.X` (+ _output_get 1))
    (`KismetSystemLibrary.DelayUntilNextTick`)
    (bind _mesh (`/Game/MarbleGame_Wallace/BluePrints/PuzzleElements/BP_ToyBall.Mesh` _asbp_toy_ball))
    (`PrimitiveComponent.AddRadialForce` _mesh (`SceneComponent.K2_GetComponentLocation` (`self.Outer`)) (`self.OuterRadius`) -8192.0 "RIF_Constant" true)
    (`KismetSystemLibrary.PrintString` (`KismetSystemLibrary.GetDisplayName` _mesh))))

(fn `UserConstructionScript`
  (`SphereComponent.SetSphereRadius` (`self.Outer`) (`self.OuterRadius`) true)
  (`SphereComponent.SetSphereRadius` (`self.Inner`) (`self.InnerRadius`) true))