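; Gate is a marble puzzle element whose Cube barrier disappears when the gate is activated.
; The Activate event disables the Cube's collision and hides it.
; With a non-zero WaitTime, it shows the Cube again after that delay but sets NoCollision again, so the reappeared gate stays passable.
; A ToggleChannel call is present but never runs.
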(event `Activate`
  (bind _cube (`self.Cube`))
  (bind _wait_time (`self.Wait time`))
  (`PrimitiveComponent.SetCollisionEnabled` _cube "NoCollision")
  (`SceneComponent.SetHiddenInGame` _cube true false)
  (if (!= _wait_time 0.0)
    (`KismetSystemLibrary.Delay` _wait_time)
    (`PrimitiveComponent.SetCollisionEnabled` _cube "NoCollision")
    (`SceneComponent.SetHiddenInGame` _cube false false)))

(fn `UserConstructionScript`)