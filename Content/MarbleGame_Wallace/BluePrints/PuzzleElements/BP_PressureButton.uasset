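; BP_PressureButton is a marble game puzzle button that triggers other elements when an actor overlaps its box.
; The overlap calls its own Activate, then activates the optional TargetBallSpawner and TargetElement if valid.
; Activate can flash the button yellow for a second before restoring its Material, which the construction script also applies along with visibility.
; A ball-only filter using LookForBall and BP_ToyBall is disconnected, so any overlapping actor triggers it.
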(event `self.Box.OnComponentBeginOverlap`
  (params (OverlappedComponent :type "PrimitiveComponent Object Reference") (OtherActor :type "Actor Object Reference") (OtherComp :type "PrimitiveComponent Object Reference") (OtherBodyIndex :type Integer) (bFromSweep :type Boolean) (SweepResult :type "HitResult Structure (by ref)"))
  (bind _target_ball_spawner (`self.Target Ball Spawner`))
  (bind _targetelement (`self.TargetElement`))
  (`self.Activate`)
  (if (`KismetSystemLibrary.IsValid` _target_ball_spawner)
    (`/Game/MarbleGame_Wallace/BluePrints/PuzzleElements/BallSpawner.Activate` _target_ball_spawner))
  (if (`KismetSystemLibrary.IsValid` _targetelement)
    (`/Game/MarbleGame_Wallace/BluePrints/PuzzleElements/BP_Element.Activate` _targetelement)))

(event `Activate`
  (bind _button (`self.Button`))
  (if (`self.DoColorToggle`)
    (`PrimitiveComponent.SetMaterial` _button 0 "/Game/Materials/MI_Yellow.MI_Yellow") ; Change the color of the platform to "Activated"
    (`KismetSystemLibrary.Delay` 1.0)
    (`PrimitiveComponent.SetMaterial` _button 0 (`self.Material`)) ; Change the color of the platform to "Activated"
  ))

(fn `UserConstructionScript`
  (`SceneComponent.SetVisibility` (`self.Button`) (`self.Visible`) false)
  (`PrimitiveComponent.SetMaterial` (`self.Button`) 0 (`self.Material`)))