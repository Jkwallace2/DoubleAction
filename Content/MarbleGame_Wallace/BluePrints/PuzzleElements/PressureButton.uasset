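; PressureButton is a puzzle-element Blueprint that activates a referenced Target when a BP_ToyBall overlaps its box trigger.
; The overlap runs the button's own Activate event, calls Activate on the Target and prints a debug string naming the receiver.
; The button's Activate swaps the mesh material, then sets GridMaterial after a short delay.
; The construction script sets button mesh visibility from a Visible variable.
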(event `self.Box.OnComponentBeginOverlap`
  (params (OverlappedComponent :type "PrimitiveComponent Object Reference") (OtherActor :type "Actor Object Reference") (OtherComp :type "PrimitiveComponent Object Reference") (OtherBodyIndex :type Integer) (bFromSweep :type Boolean) (SweepResult :type "HitResult Structure (by ref)"))
  (cast `/Game/MarbleGame_Wallace/BluePrints/PuzzleElements/BP_ToyBall` OtherActor)
  (`self.Activate`)
  (`/Game/MarbleGame_Wallace/BluePrints/PuzzleElements/BP_Element.Activate` (`self.Target`))
  (`KismetSystemLibrary.PrintString` (`KismetStringLibrary.Concat_StrStr` "sending data to " (`KismetSystemLibrary.GetDisplayName` null))))

(event `Activate`
  (bind _button (`self.Button`))
  (`PrimitiveComponent.SetMaterial` _button 0 null) ; Change the color of the platform to "Activated"
  (`KismetSystemLibrary.Delay` 1.0)
  (`PrimitiveComponent.SetMaterial` _button 0 "/Engine/EditorMaterials/GridMaterial.GridMaterial") ; Change the color of the platform to "Activated"
)

(fn `UserConstructionScript`
  (`SceneComponent.SetVisibility` (`self.Button`) (`self.Visible`) false))