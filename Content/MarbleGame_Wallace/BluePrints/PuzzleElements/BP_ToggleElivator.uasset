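; BP_ToggleElivator is a puzzle-element elevator that, once activated, shuttles back and forth continuously.
; Activate plays a Timeline whose float track lerps the Cube's relative location between the Start and End components, without sweeping.
; Each time the Timeline finishes, a short Delay feeds a FlipFlop that alternates reversing from the end and playing from the start, with no stop logic.
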(event `self.Activate`
  (bind (_direction _floattrack) (`Timeline|Timeline` :!label _label)
    (:`Update`
      (`SceneComponent.K2_SetRelativeLocation` (`self.Cube`) (`KismetMathLibrary.VLerp` (`SceneComponent.RelativeLocation` (`self.Start`)) (`SceneComponent.RelativeLocation` (`self.End`)) _floattrack) false false))
    (:`Finished`
      (`KismetSystemLibrary.Delay` 2.0)
      (`/Engine/EditorBlueprintResources/StandardMacros.FlipFlop` ; If A, Reverse from End\nif B, Start from Beginning
        (:`A`
          (goto _label :!via `ReverseFromEnd`))
        (:`B`
          (goto _label :!via `PlayFromStart`))))))

(fn `UserConstructionScript`
  (`parent.UserConstructionScript`))