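; Ball dispenser puzzle element for a marble game that releases a toy ball when activated.
; Activate plays a sound, spawns one ball in place of the display sphere, and swings two arms through two chained timelines, ignoring retriggers until finished.
; A box overlap records the latest toy ball as MyKid.
; Reset kills that ball if valid, then restores the sphere and re-arms the do-once spawn.
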(event `Activate`
  (bind _sm_arm_ld1 (`self.SM_Arm_LD1`))
  (bind _sm_arm_ld (`self.SM_Arm_LD`))
  (bind _returnvalue (`SceneComponent.K2_GetComponentLocation` (`self.DefaultSceneRoot`)))
  (bind (_relativerotation_roll _relativerotation_pitch _relativerotation_yaw) (`KismetMathLibrary.BreakRotator` (`SceneComponent.RelativeRotation` _sm_arm_ld1)))
  (bind (_relativerotation_roll_2 _relativerotation_pitch_2 _relativerotation_yaw_2) (`KismetMathLibrary.BreakRotator` (`SceneComponent.RelativeRotation` _sm_arm_ld)))
  (if (not (`self.Activated`))
    (set `self.Activated` true)
    (`GameplayStatics.PlaySoundAtLocation` null _returnvalue (struct) 1.0 1.0 0.0 null null null null)
    (`self.SpawnBall`)
    (bind (_direction _newtrack_1) (`Timeline|Timeline` :!via `PlayFromStart`)
      (:`Update`
        (bind _returnvalue_2 (* _newtrack_1 80.0))
        (`SceneComponent.K2_SetRelativeRotation` _sm_arm_ld (`KismetMathLibrary.MakeRotator` _relativerotation_roll_2 _returnvalue_2 _relativerotation_yaw_2) false false)
        (`SceneComponent.K2_SetRelativeRotation` _sm_arm_ld1 (`KismetMathLibrary.MakeRotator` _relativerotation_roll _returnvalue_2 _relativerotation_yaw) false false))
      (:`Finished`
        (`KismetSystemLibrary.Delay` 0.1)
        (bind (_direction_2 _newtrack_1_2) (`Timeline|Timeline_0` :!via `PlayFromStart`)
          (:`Update`
            (bind _returnvalue_3 (* _newtrack_1_2 80.0))
            (`SceneComponent.K2_SetRelativeRotation` _sm_arm_ld1 (`KismetMathLibrary.MakeRotator` _relativerotation_roll _returnvalue_3 _relativerotation_yaw) false false)
            (`SceneComponent.K2_SetRelativeRotation` _sm_arm_ld (`KismetMathLibrary.MakeRotator` _relativerotation_roll_2 _returnvalue_3 _relativerotation_yaw_2) false false))
          (:`Finished`
            (`GameplayStatics.PlaySoundAtLocation` null _returnvalue (struct) 1.0 1.0 0.0 null null null null)
            (set `self.Activated` false)))))))

(event `SpawnBall`
  ;[1 1 1] Spawn Ball
  (`/Engine/EditorBlueprintResources/StandardMacros.DoOnce` false :!label _label
    (:`Completed`
      (`SceneComponent.SetVisibility` (`self.Sphere`) false false)
      (`|SpawnActorFromClass` (`self.ToyBall`) (`KismetMathLibrary.Conv_VectorToTransform` (`SceneComponent.K2_GetComponentLocation` (`self.DefaultSceneRoot`))) "Undefined" "MultiplyWithRoot" null null)
      (`KismetSystemLibrary.PrintText` "Ball Spawned!"))))

(event `self.Box.OnComponentBeginOverlap`
  (params (OverlappedComponent :type "PrimitiveComponent Object Reference") (OtherActor :type "Actor Object Reference") (OtherComp :type "PrimitiveComponent Object Reference") (OtherBodyIndex :type Integer) (bFromSweep :type Boolean) (SweepResult :type "HitResult Structure (by ref)"))
  (bind _asbp_toy_ball (cast `/Game/MarbleGame_Wallace/BluePrints/PuzzleElements/BP_ToyBall` OtherActor))
  (set `self.my kid` _asbp_toy_ball))

(event `Reset`
  (bind _my_kid (`self.my kid`))
  (if (`KismetSystemLibrary.IsValid` _my_kid)
    (`/Game/MarbleGame_Wallace/BluePrints/PuzzleElements/BP_ToyBall.CommitDie` _my_kid)
    ;[1 1 1] Spawn Ball
    (`SceneComponent.SetVisibility` (`self.Sphere`) true false)
    (goto _label :!via `Reset`)))

(fn `UserConstructionScript`
  (bind _sphere (`self.Sphere`))
  (set `self.My Balls` 0)
  (`SceneComponent.SetVisibility` _sphere true false)
  (`PrimitiveComponent.SetMaterial` _sphere 0 (`self.Material`)))